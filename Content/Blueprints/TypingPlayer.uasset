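; TypingPlayer is a player Blueprint that sets up typing UI and captures keyboard input.
; On BeginPlay it creates two widgets, a key log and a TextInput box, and adds both to the viewport.
; Any key press appends that key's display name to a running InputText string, which is sent to the key log.
; Space bar tells the text box to change word and focuses its editable field.
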(event `Key|SpaceBar`
  (params (Key :type "Key Structure"))
  (bind _textbox (`self.TextBox`))
  (:`Pressed`
    (`/Game/Blueprints/TextInput.ChangeWord` _textbox)
    (`Widget.SetFocus` (`/Game/Blueprints/TextInput.EditableTextBox_24` _textbox))))

(event `self.ReceiveBeginPlay`
  (bind _returnvalue (`|CreateWidget` "/Game/Blueprints/KeyLog.KeyLog_C"))
  (bind _output_get (set `self.LoggedKeys` _returnvalue))
  (`UserWidget.AddToViewport` _output_get 0)
  (bind _returnvalue_2 (`|CreateWidget` "/Game/Blueprints/TextInput.TextInput_C"))
  (bind _output_get_2 (set `self.TextBox` _returnvalue_2))
  (`UserWidget.AddToViewport` _output_get_2 0))

(event `Key|AnyKey`
  (params (Key :type "Key Structure"))
  (:`Pressed`
    (bind _output_get (set `self.InputText` (`KismetTextLibrary.Conv_StringToText` (`KismetStringLibrary.Concat_StrStr` (`KismetTextLibrary.Conv_TextToString` (`self.InputText`)) " " (`KismetTextLibrary.Conv_TextToString` (`KismetInputLibrary.Key_GetDisplayName` Key))))))
    (`/Game/Blueprints/KeyLog.SetKey` (`self.LoggedKeys`) _output_get)))

(fn `UserConstructionScript`)