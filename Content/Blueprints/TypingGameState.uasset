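; Game state for a typing game that supplies the quote and tracks when every player has finished.
; On begin play it picks a random row from the Quotes data table and resets the finish state.
; Switching screens moves each player's TypingController to the game and runs a timeline that updates an integer countdown.
; Finish reports increment a count, and GameFinished is set once it equals the player count.
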(event `self.ReceiveBeginPlay`
  (`self.NewQuote`))

(event `NewQuote`
  (bind _returnvalue (`|GetDataTableRow` (`self.Quotes`) (`KismetStringLibrary.Conv_StringToName` (`KismetStringLibrary.Conv_IntToString` (`KismetMathLibrary.RandomIntegerInRange` 1 38000))))
    (:`then`
      (set `self.CurrentQuote` (`.Quote_12_BF78E768470D96FA5F36D18A71BC04ED` (break `/Game/Data/Quote_Struct` _returnvalue)))
      (set `self.GameFinished` false)
      (set `self.FinishedCount` 0))))

(event `IncreaseNumber`
  (`/Engine/EditorBlueprintResources/StandardMacros.IncrementInt` (`self.Number`)))

(event `SwitchScreen`
  (params (Index :type Integer))
  (for _array_element (`self.PlayerArray`)
    (bind _astyping_controller (cast `/Game/Blueprints/TypingController` (`self.GetOwner` _array_element)))
    (`/Game/Blueprints/TypingController.SwitchToGame` _astyping_controller 1))
  (bind (_direction _newtrack_0) (`Timeline|Timeline_0` :!via `PlayFromStart`)
    (:`Update`
      (set `self.Countdown` (`KismetMathLibrary.FTrunc` _newtrack_0)))))

(event `PlayerFinished`
  (bind _result (`/Engine/EditorBlueprintResources/StandardMacros.IncrementInt` (`self.FinishedCount`))
    (:`  `
      (if (== _result (`KismetArrayLibrary.Array_Length` (`self.PlayerArray`)))
        (set `self.GameFinished` true)))))

(fn `UserConstructionScript`)