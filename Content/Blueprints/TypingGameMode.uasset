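; TypingGameMode is the game mode that sets up the lobby for each player who joins the typing game.
; On PostLogin it records the new player in a unique Players list and fetches the game instance through a reference message.
; It then gets the player's lobby reference, runs its initial setup and builds the lobby menu with the server name.
; Finally, it tells TypingGameState to list the players.
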(event `self.K2_PostLogin`
  (params (NewPlayer :type "PlayerController Object Reference"))
  (`KismetSystemLibrary.PrintString` "Hello")
  (`KismetArrayLibrary.Array_AddUnique` (`self.Players`) NewPlayer)
  (bind _typinggameinstance (message `/Game/Blueprints/Menu/BTI_GameInstance.TypingGameInstanceRef` (`GameplayStatics.GetGameInstance`)))
  (bind _output_get (set `self.GameInstance` _typinggameinstance))
  (bind _playercontroller (message `/Game/Blueprints/BTI_Lobby.LobbyRef` NewPlayer))
  (`/Game/Blueprints/TypingController.InitialSetup` _playercontroller)
  (`/Game/Blueprints/TypingController.SetupLobbyMenu` _playercontroller (`/Game/Blueprints/TypingGameInstance.ServerName` _output_get))
  (bind _astyping_game_state (cast `/Game/Blueprints/TypingGameState` (`GameplayStatics.GetGameState`)))
  (`/Game/Blueprints/TypingGameState.ListPlayers` _astyping_game_state))

(fn `UserConstructionScript`)