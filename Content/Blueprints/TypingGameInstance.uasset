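; Game instance for a typing game that manages top-level UI and session teardown.
; Events create and cache the main menu and loading screen widgets, show the mouse cursor with the menu, and toggle its quit prompt.
; Network and travel failures feed the ErrorMessage graph, which replaces any visible error widget with a new one showing the failure type.
; A separate event destroys the session for a given player controller.
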(event `/Game/Blueprints/Menu/BTI_GameInstance.ShowMainMenu`
  ;[1 1 1] MainMenu
  (bind _mainwidget (`self.MainWidget`)
    (:`then`
      (if (not (`Widget.IsInViewport` _mainwidget))
        (`UserWidget.AddToViewport` (stale _output_get) 0 :!label _label)))
    (:`else`
      (bind _returnvalue (`|CreateWidget` "/Game/Widgets/UI_Main.UI_Main_C" (`GameplayStatics.GetPlayerController` 0)))
      (bind _output_get (set `self.MainWidget` _returnvalue))
      (goto _label)))
  (set `PlayerController.bShowMouseCursor` true (`GameplayStatics.GetPlayerController` 0)))

(event `self.HandleNetworkError`
  (params (FailureType :type "ENetworkFailure Enum" :default "NetDriverAlreadyExists") (bIsServer :type Boolean))
  ;[1 1 1] Errors
  (`self.ErrorMessage` (`|GetEnumeratorNameAsString` FailureType)))

(event `self.HandleTravelError`
  (params (FailureType :type "ETravelFailure Enum" :default "NoLevel"))
  ;[1 1 1] Errors
  (`self.ErrorMessage` (`|GetEnumeratorNameAsString` FailureType)))

(event `/Game/Blueprints/Menu/BTI_GameInstance.ShowQuit`
  ;[1 1 1] QuitGame
  (bind _mainwidget (`self.MainWidget`)
    (:`then`
      (`/Game/Widgets/UI_Main.OpenCloseQuit` _mainwidget))
    (:`else`)))

(event `/Game/Blueprints/Menu/BTI_GameInstance.ShowLoadingScreen`
  ;[1 1 1] Loading Screen
  (`self.LoadingScreenWidget`
    (:`then`
      _)
    (:`else`
      (bind _returnvalue (`|CreateWidget` "/Game/Blueprints/Menu/UI_LoadingScreen.UI_LoadingScreen_C" (`GameplayStatics.GetPlayerController` 0)))
      (bind _output_get (set `self.LoadingScreenWidget` _returnvalue))))
  (`UserWidget.AddToViewport` _output_get 0))

(event `/Game/Blueprints/Menu/BTI_GameInstance.DestroySessionCaller`
  (params (PlayerController :type "PlayerController Object Reference"))
  ;[1 1 1] Destroy Session
  (`DestroySessionCallbackProxy.DestroySession` PlayerController))

(fn `TypingGameInstanceRef`
  (returns (TypingGameInstance :type "/Game/Blueprints/TypingGameInstance Object Reference"))
  (return self))